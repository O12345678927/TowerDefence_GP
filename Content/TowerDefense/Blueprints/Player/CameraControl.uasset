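; Player controller for the tower defense game that turns mouse and keyboard input into camera pan and zoom flags and toggles the pause menu.
; BeginPlay shows and locks the cursor, enables click events and caches the CameraChar, whose movement flags it sets.
; Screen-edge mouse detection pans, while held WASD or arrow keys set BlockMouse so mouse movement cannot cancel them.
; P toggles pause through the player character's TD_GameMgnrActorComp and a PauseMenu widget.
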(event `self.ReceiveBeginPlay`
  ;[1 1 1] Set Input
  (set `self.bShowMouseCursor` true)
  (`WidgetBlueprintLibrary.SetInputMode_GameAndUIEx` self null "LockAlways")
  ;[1 1 1] Cache Camera Char
  (bind _returnvalue (`GameplayStatics.GetActorOfClass` "/Game/TowerDefense/Blueprints/Player/CameraChar.CameraChar_C"))
  (set `self.CameraCharacter` _returnvalue)
  ;[1 1 1] Click events
  (set `self.bEnableClickEvents` true))

(event `InputAxisKey|MouseX`
  (params (AxisValue :type "Float (single-precision)"))
  (bind _returnvalue_x (`KismetMathLibrary.BreakVector2D` (`WidgetLayoutLibrary.GetViewportSize`)))
  (bind _blockmouse (`self.BlockMouse`))
  (bind _cameracharacter (`self.CameraCharacter`))
  (bind _returnvalue (/ (`self.GetMousePosition` self) _returnvalue_x))
  ;[1 1 1] Set Mouse X Edge Detect
  ;;[1 1 1] Detect edge
  (if (> _returnvalue 0.98)
    ;;[1 1 1] Movement
    (set `/Game/TowerDefense/Blueprints/Player/CameraChar.MoveRight` true _cameracharacter :!label _label)
    (else
      (`|ExecutionSequence`
        (:`then_0`
          ;;[1 1 1] Block mouse for keyboard
          (if (not _blockmouse)
            (set `/Game/TowerDefense/Blueprints/Player/CameraChar.MoveRight` false _cameracharacter :!label _label_2)))
        (:`then_1`
          (if (< _returnvalue 0.02)
            (set `/Game/TowerDefense/Blueprints/Player/CameraChar.MoveLeft` true _cameracharacter :!label _label_3)
            (elif (not _blockmouse)
              (set `/Game/TowerDefense/Blueprints/Player/CameraChar.MoveLeft` false _cameracharacter :!label _label_4))))))))

(event `Key|D`
  (params (Key :type "Key Structure"))
  ;[1 1 1] Keyboard input override
  (:`Pressed`
    (set `self.BlockMouse` true :!label _label_5)
    (goto _label))
  (:`Released`
    (set `self.BlockMouse` false :!label _label_6)
    (goto _label_2)))

(event `Key|Right`
  (params (Key :type "Key Structure"))
  ;[1 1 1] Keyboard input override
  (:`Pressed`
    (goto _label_5))
  (:`Released`
    (goto _label_6)))

(event `Key|A`
  (params (Key :type "Key Structure"))
  ;[1 1 1] Keyboard input override
  (:`Pressed`
    (set `self.BlockMouse` true :!label _label_7)
    (goto _label_3))
  (:`Released`
    (set `self.BlockMouse` false :!label _label_8)
    (goto _label_4)))

(event `Key|Left`
  (params (Key :type "Key Structure"))
  ;[1 1 1] Keyboard input override
  (:`Pressed`
    (goto _label_7))
  (:`Released`
    (goto _label_8)))

(event `InputAxisKey|MouseY`
  (params (AxisValue :type "Float (single-precision)"))
  (bind (_returnvalue_x _returnvalue_y) (`KismetMathLibrary.BreakVector2D` (`WidgetLayoutLibrary.GetViewportSize`)))
  (bind _blockmouse (`self.BlockMouse`))
  (bind _cameracharacter (`self.CameraCharacter`))
  (bind _returnvalue (/ (`.LocationY` (`self.GetMousePosition` self)) _returnvalue_y))
  ;[1 1 1] Set Mouse Y Edge Detect
  ;;[1 1 1] Detect edge
  (if (> _returnvalue 0.98)
    ;;[1 1 1] Movement
    (set `/Game/TowerDefense/Blueprints/Player/CameraChar.MoveDown` true _cameracharacter :!label _label_9)
    (else
      (`|ExecutionSequence`
        (:`then_0`
          ;;[1 1 1] Block mouse for keyboard
          (if (not _blockmouse)
            (set `/Game/TowerDefense/Blueprints/Player/CameraChar.MoveDown` false _cameracharacter :!label _label_10)))
        (:`then_1`
          (if (< _returnvalue 0.02)
            (set `/Game/TowerDefense/Blueprints/Player/CameraChar.MoveUp` true _cameracharacter :!label _label_11)
            (elif (not _blockmouse)
              (set `/Game/TowerDefense/Blueprints/Player/CameraChar.MoveUp` false _cameracharacter :!label _label_12))))))))

(event `Key|Add`
  (params (Key :type "Key Structure"))
  (bind _cameracharacter (`self.CameraCharacter`))
  ;[1 1 1] Camera Zoom input
  (:`Pressed`
    (set `/Game/TowerDefense/Blueprints/Player/CameraChar.MoveIn` true _cameracharacter :!label _label_13))
  (:`Released`
    (set `/Game/TowerDefense/Blueprints/Player/CameraChar.MoveIn` false _cameracharacter :!label _label_14)))

(event `Key|S`
  (params (Key :type "Key Structure"))
  ;[1 1 1] Keyboard input override
  (:`Pressed`
    (set `self.BlockMouse` true :!label _label_15)
    (goto _label_9))
  (:`Released`
    (set `self.BlockMouse` false :!label _label_16)
    (goto _label_10)))

(event `Key|E`
  (params (Key :type "Key Structure"))
  ;[1 1 1] Camera Zoom input
  (:`Pressed`
    (goto _label_13))
  (:`Released`
    (goto _label_14)))

(event `Key|Down`
  (params (Key :type "Key Structure"))
  ;[1 1 1] Keyboard input override
  (:`Pressed`
    (goto _label_15))
  (:`Released`
    (goto _label_16)))

(event `Key|Subtract`
  (params (Key :type "Key Structure"))
  (bind _cameracharacter (`self.CameraCharacter`))
  ;[1 1 1] Camera Zoom input
  (:`Pressed`
    (set `/Game/TowerDefense/Blueprints/Player/CameraChar.MoveOut` true _cameracharacter :!label _label_17))
  (:`Released`
    (set `/Game/TowerDefense/Blueprints/Player/CameraChar.MoveOut` false _cameracharacter :!label _label_18)))

(event `Key|Q`
  (params (Key :type "Key Structure"))
  ;[1 1 1] Camera Zoom input
  (:`Pressed`
    (goto _label_17))
  (:`Released`
    (goto _label_18)))

(event `Key|W`
  (params (Key :type "Key Structure"))
  ;[1 1 1] Keyboard input override
  (:`Pressed`
    (set `self.BlockMouse` true :!label _label_19)
    (goto _label_11))
  (:`Released`
    (set `self.BlockMouse` false :!label _label_20)
    (goto _label_12)))

(event `Key|Up`
  (params (Key :type "Key Structure"))
  ;[1 1 1] Keyboard input override
  (:`Pressed`
    (goto _label_19))
  (:`Released`
    (goto _label_20)))

(event `Key|P` :paused true
  (params (Key :type "Key Structure"))
  (bind _returnvalue (`self.GetComponentByClass` (`GameplayStatics.GetPlayerCharacter` 0) "/Game/TowerDefense/Blueprints/Player/TD_GameMgnrActorComp.TD_GameMgnrActorComp_C"))
  ;[1 1 1] Pause Game
  (:`Pressed`
    (if (not (`/Game/TowerDefense/Blueprints/Player/TD_GameMgnrActorComp.GamePaused` _returnvalue))
      (bind _output_get (set `/Game/TowerDefense/Blueprints/Player/TD_GameMgnrActorComp.GamePaused` true _returnvalue))
      (bind _returnvalue_2 (`|CreateWidget` "/Game/TowerDefense/Blueprints/Widgets/PauseMenu.PauseMenu_C" self))
      (bind _output_get_2 (set `self.PauseMenuWidget` _returnvalue_2))
      (`UserWidget.AddToViewport` _output_get_2 0)
      (`GameplayStatics.SetGamePaused` _output_get)
      (else
        (bind _output_get_3 (set `/Game/TowerDefense/Blueprints/Player/TD_GameMgnrActorComp.GamePaused` false _returnvalue))
        (`Widget.RemoveFromParent` (`self.PauseMenuWidget`))
        (`GameplayStatics.SetGamePaused` _output_get_3)))))

(fn `UserConstructionScript`)