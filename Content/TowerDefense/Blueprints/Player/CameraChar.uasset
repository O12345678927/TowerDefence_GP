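; CameraChar is a tower defense player camera actor that scrolls along the world axes within a bounded volume around its start location.
; BeginPlay records the start position and derives negated speed and range values.
; Each Tick first clears any Move flag whose direction has passed its bound, then offsets the actor by delta-scaled ScrollSpeed for the flags still set.
; The six direction flags are only cleared here, never set.
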(event `self.ReceiveBeginPlay`
  (bind _returnvalue_location (`KismetMathLibrary.BreakTransform` (`self.GetTransform` self)))
  ;[1 1 1] Set Values
  (set `self.ScrollSpeedNegative` (* (`self.ScrollSpeed`) -1.0))
  (set `self.BRNeg_LeftRight` (* (`self.BoundsRangeLeftRight`) -1.0))
  (set `self.BRNeg_UpDown` (* (`self.BoundsRangeUpDown`) -1.0))
  (set `self.BRNeg_InOut` (* (`self.BoundsRangeInOut`) -1.0))
  (set `self.StartPos` _returnvalue_location))

(event `self.ReceiveTick`
  (params (DeltaSeconds :type "Float (single-precision)"))
  (bind _returnvalue_location (`KismetMathLibrary.BreakTransform` (`self.GetTransform` self)))
  (bind _returnvalue (* DeltaSeconds (`self.ScrollSpeedNegative`)))
  (bind _returnvalue_2 (* DeltaSeconds (`self.ScrollSpeed`)))
  (bind (_returnvalue_x _returnvalue_y _returnvalue_z) (`KismetMathLibrary.BreakVector` (- _returnvalue_location (`self.StartPos`))))
  ;[1 1 1] Move Camera
  (`|ExecutionSequence`
    (:`then_0`
      ;[1 1 1] Camera Bounds
      (`|ExecutionSequence`
        (:`then_0`
          (if (> _returnvalue_x (`self.BoundsRangeUpDown`))
            (set `self.MoveUp` false)))
        (:`then_1`
          (if (< _returnvalue_x (`self.BRNeg_UpDown`))
            (set `self.MoveDown` false)))
        (:`then_2`
          (if (> _returnvalue_y (`self.BoundsRangeLeftRight`))
            (set `self.MoveRight` false)))
        (:`then_3`
          (if (< _returnvalue_y (`self.BRNeg_LeftRight`))
            (set `self.MoveLeft` false)))
        (:`then_4`
          (if (> _returnvalue_z (`self.BoundsRangeInOut`))
            (set `self.MoveOut` false)))
        (:`then_5`
          (if (< _returnvalue_z (`self.BRNeg_InOut`))
            (set `self.MoveIn` false)))))
    (:`then_1`
      (`|ExecutionSequence`
        (:`then_0`
          (if (`self.MoveLeft`)
            (`self.K2_AddActorWorldOffset` (`KismetMathLibrary.MakeVector` 0.0 _returnvalue))))
        (:`then_1`
          (if (`self.MoveRight`)
            (`self.K2_AddActorWorldOffset` (`KismetMathLibrary.MakeVector` 0.0 _returnvalue_2))))
        (:`then_2`
          (if (`self.MoveUp`)
            (`self.K2_AddActorWorldOffset` (`KismetMathLibrary.MakeVector` _returnvalue_2))))
        (:`then_3`
          (if (`self.MoveDown`)
            (`self.K2_AddActorWorldOffset` (`KismetMathLibrary.MakeVector` _returnvalue))))
        (:`then_4`
          (if (`self.MoveIn`)
            (`self.K2_AddActorWorldOffset` (`KismetMathLibrary.MakeVector` 0.0 0.0 _returnvalue))))
        (:`then_5`
          (if (`self.MoveOut`)
            (`self.K2_AddActorWorldOffset` (`KismetMathLibrary.MakeVector` 0.0 0.0 _returnvalue_2))))))))

(fn `UserConstructionScript`)