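; Tower defense enemy character that walks numbered PathPoint actors to the player base, damaging it and destroying itself on overlap.
; Overlaps advance the checkpoint index, matched against numbers parsed from actor display names, with SimpleMoveToActor handling movement.
; Health scales by a per-wave increment from the player's game manager component, which receives alive and kill counts.
; Tick updates the health bar widget, heads for the base after the last point, and awards death money.
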(event `self.CapsuleComponent.OnComponentBeginOverlap`
  (params (OverlappedComponent :type "PrimitiveComponent Object Reference") (OtherActor :type "Actor Object Reference") (OtherComp :type "PrimitiveComponent Object Reference") (OtherBodyIndex :type Integer) (bFromSweep :type Boolean) (SweepResult :type "HitResult Structure (by ref)"))
  (bind _gamemanager (`self.GameManager`))
  ;[1 1 1] Check for hit
  (`|ExecutionSequence`
    (:`then_0`
      ;[0.5312 0.02453 0] Damage Player Base
      ;;[1 1 1] Check if enemy
      (`/Engine/EditorBlueprintResources/StandardMacros.IsValid` OtherActor
        (:`Is Valid`
          (if (`self.ActorHasTag` OtherActor "Base")
            ;;[1 1 1] Apply damage
            (bind _returnvalue (`GameplayStatics.ApplyDamage` OtherActor (`self.PlayerBaseDamage`)))
            (`KismetSystemLibrary.PrintString` (`KismetStringLibrary.Concat_StrStr` "damaged base | HP: " (`KismetStringLibrary.Conv_DoubleToString` _returnvalue)) true true (struct :`R` 1.0 :`G` 0.06348 :`A` 1.0))
            ;;[1 1 1] Set enemies this wave (kills)
            (set `/Game/TowerDefense/Blueprints/Player/TD_GameMgnrActorComp.Kills` (+ (`/Game/TowerDefense/Blueprints/Player/TD_GameMgnrActorComp.Kills` _gamemanager) 1.0) _gamemanager)
            (`self.K2_DestroyActor`)))))
    (:`then_1`
      ;[1 1 1] Find Checkpoints & Move
      ;;[1 1 1] if checkpoint
      (`/Engine/EditorBlueprintResources/StandardMacros.IsValid` OtherActor
        (:`Is Valid`
          (if (`self.ActorHasTag` OtherActor "PathPoint")
            ;;[1 1 1] move to next checkpoint
            (set `self.CheckpointIndex` (+ (`self.CheckpointIndex`) 1))
            ;;[1 1 1] Find checkpoints
            (for _array_element (stale `self.ReceiveBeginPlay` _outactors) :!label _label
              ;;[1 1 1] Check if correct checkpoint to move to
              (if (== (`KismetStringLibrary.Conv_StringToInt` (`KismetStringLibrary.RightChop` (`KismetSystemLibrary.GetDisplayName` _array_element) 9)) (`self.CheckpointIndex`))
                ;;[1 1 1] move
                (`AIBlueprintHelperLibrary.SimpleMoveToActor` (`self.GetController`) _array_element)))))))))

(event `self.ReceiveAnyDamage`
  (params (Damage :type "Float (single-precision)") (DamageType :type "DamageType Object Reference") (InstigatedBy :type "Controller Object Reference") (DamageCauser :type "Actor Object Reference"))
  (bind _enemyhealth (`self.EnemyHealth`))
  (set `self.EnemyHealth` (- _enemyhealth Damage))
  (if (<= _enemyhealth 0.0)
    (`/Engine/EditorBlueprintResources/StandardMacros.IncrementFloat` (`/Game/TowerDefense/Blueprints/Player/TD_GameMgnrActorComp.Kills` (`self.GameManager`))
      (:`  `
        (`self.K2_DestroyActor`)))))

(event `self.ReceiveBeginPlay`
  (bind _gamemanager (`self.GameManager`))
  ;[1 1 1] Set max health
  (set `self.GameManager` (`self.GetComponentByClass` (`GameplayStatics.GetPlayerCharacter` 0) "/Game/TowerDefense/Blueprints/Player/TD_GameMgnrActorComp.TD_GameMgnrActorComp_C"))
  (`|ExecutionSequence`
    (:`then_0`
      (set `self.EnemyHealth` (+ (`self.EnemyHealth`) (`/Game/TowerDefense/Blueprints/Player/TD_GameMgnrActorComp.EnemyHealthIncPerWave` _gamemanager)))
      (set `self.MaxHealth` (`self.EnemyHealth`))
      ;[1 1 1] Initialize
      (`self.SpawnDefaultController`)
      (set `self.Tags` (`self.Tags`))
      ;[1 1 1] Find Checkpoints & Move
      ;;[1 1 1] Find checkpoints
      (bind _outactors (`GameplayStatics.GetAllActorsOfClass` "/Game/TowerDefense/Blueprints/Game/PathPoint0.PathPoint0_C"))
      (set `self.Checkpoints` _outactors)
      (goto _label))
    (:`then_1`
      ;[1 1 1] Disable Health Bar Shadow
      (`PrimitiveComponent.SetCastShadow` (`self.EnemyHealthBarWidget`) false))
    (:`then_2`
      ;[1 1 1] Set enemies alive
      (set `/Game/TowerDefense/Blueprints/Player/TD_GameMgnrActorComp.EnemiesAliveThisWave` (+ (`/Game/TowerDefense/Blueprints/Player/TD_GameMgnrActorComp.EnemiesAliveThisWave` _gamemanager) 1) _gamemanager))))

(event `self.ReceiveTick`
  (params (DeltaSeconds :type "Float (single-precision)"))
  (bind _enemyhealthbarwidget (`self.EnemyHealthBarWidget`))
  (bind (_returnvalue_x _returnvalue_y _returnvalue_z) (`KismetMathLibrary.BreakVector` (`SceneComponent.K2_GetComponentLocation` _enemyhealthbarwidget)))
  (bind _returnvalue (`self.GetComponentByClass` (`GameplayStatics.GetPlayerCharacter` 0) "/Game/TowerDefense/Blueprints/Player/TD_GameMgnrActorComp.TD_GameMgnrActorComp_C"))
  (bind _returnvalue_2 (`WidgetComponent.GetWidget` (`self.EnemyHealthBarWidget`)))
  (bind (_returnvalue_x_2 _returnvalue_y_2 _returnvalue_z_2) (`KismetMathLibrary.BreakVector` (`SceneComponent.K2_GetComponentLocation` (`PlayerCameraManager.TransformComponent` (`GameplayStatics.GetPlayerCameraManager` 0)))))
  ;[1 1 1] update
  (`|ExecutionSequence`
    (:`then_0`
      ;[1 1 1] Move To Base
      ;;[1 1 1] check if past last point
      (if (== (`self.CheckpointIndex`) (`KismetArrayLibrary.Array_Length` (`self.Checkpoints`)))
        (`/Engine/EditorBlueprintResources/StandardMacros.DoOnce` false
          (:`Completed`
            ;;[1 1 1] move
            (bind _returnvalue_3 (`GameplayStatics.GetActorOfClass` "/Game/TowerDefense/Blueprints/Game/PlayerBase.PlayerBase_C"))
            (`AIBlueprintHelperLibrary.SimpleMoveToActor` (`self.GetController`) _returnvalue_3)))))
    (:`then_1`
      ;[1 1 1] Enemy Health Bar
      ;;[1 1 1] Get enemy health bar widget
      (`/Engine/EditorBlueprintResources/StandardMacros.IsValid` _returnvalue_2
        (:`Is Valid`
          (bind _asenemy_health_bar_ui (cast `/Game/TowerDefense/Blueprints/Widgets/EnemyHealthBarUI` _returnvalue_2))
          ;;[1 1 1] Set percent
          (`ProgressBar.SetPercent` (`/Game/TowerDefense/Blueprints/Widgets/EnemyHealthBarUI.ProgressBar_EnemyHP` _asenemy_health_bar_ui) (/ (`self.EnemyHealth`) (`self.MaxHealth`)))
          (`SceneComponent.K2_SetWorldRotation` _enemyhealthbarwidget (`KismetMathLibrary.FindLookAtRotation` (`KismetMathLibrary.MakeVector` 0.0 0.0 _returnvalue_z) (`KismetMathLibrary.MakeVector` 0.0 0.0 _returnvalue_z_2)) false false))))
    (:`then_2`
      ;[1 0 0] Kill Enemy
      ;;[1 1 1] check if dead
      (if (<= (`self.EnemyHealth`) 0.0)
        ;;[1 1 1] set enemies this wave (kills) and money to reward on kill
        (set `/Game/TowerDefense/Blueprints/Player/TD_GameMgnrActorComp.Kills` (+ (`/Game/TowerDefense/Blueprints/Player/TD_GameMgnrActorComp.Kills` _returnvalue) 1.0) _returnvalue)
        (set `/Game/TowerDefense/Blueprints/Player/TD_GameMgnrActorComp.Money` (+ (`self.MoneyToRewardOnKill`) (`/Game/TowerDefense/Blueprints/Player/TD_GameMgnrActorComp.Money` _returnvalue)) _returnvalue)))))

(fn `UserConstructionScript`)