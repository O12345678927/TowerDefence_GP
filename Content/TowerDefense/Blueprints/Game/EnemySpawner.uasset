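; Tower defense spawner actor that spawns waves of enemies at its own transform, hiding its marker cube on play.
; Tick sets DontSpawn on the player character's game manager component when the wave's enemy count equals its kill target.
; A zero count starts a self-looping Delay chain that spawns from EnemiesToSpawn until DontSpawn is set.
; SpawningMode picks the manager's indexed type, a random entry, or sequential entries via a local index.
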(event `self.ReceiveTick`
  (params (DeltaSeconds :type "Float (single-precision)"))
  (bind _returnvalue (`self.GetComponentByClass` (`GameplayStatics.GetPlayerCharacter` 0) "/Game/TowerDefense/Blueprints/Player/TD_GameMgnrActorComp.TD_GameMgnrActorComp_C"))
  (bind _enemiestospawn (`/Game/TowerDefense/Blueprints/Player/TD_GameMgnrActorComp.EnemiesToSpawn` _returnvalue))
  (bind _enemiestospawn_2 (`/Game/TowerDefense/Blueprints/Player/TD_GameMgnrActorComp.EnemiesToSpawn` _returnvalue))
  (bind _enemiesalivethiswave (`/Game/TowerDefense/Blueprints/Player/TD_GameMgnrActorComp.EnemiesAliveThisWave` _returnvalue))
  (bind _dontspawn (`/Game/TowerDefense/Blueprints/Player/TD_GameMgnrActorComp.DontSpawn` _returnvalue))
  (bind _enemiestospawn_3 (`/Game/TowerDefense/Blueprints/Player/TD_GameMgnrActorComp.EnemiesToSpawn` _returnvalue))
  ;[1 1 1] Check if wave is/not done
  (`|ExecutionSequence`
    (:`then_0`
      (if (== (`KismetMathLibrary.FCeil` (`/Game/TowerDefense/Blueprints/Player/TD_GameMgnrActorComp.KillsToWinWave` _returnvalue)) _enemiesalivethiswave)
        (set `/Game/TowerDefense/Blueprints/Player/TD_GameMgnrActorComp.DontSpawn` true _returnvalue)
        (else
          (set `/Game/TowerDefense/Blueprints/Player/TD_GameMgnrActorComp.DontSpawn` false _returnvalue))))
    (:`then_1`
      (if (== 0 _enemiesalivethiswave)
        (switch `/Game/TowerDefense/Blueprints/Game/SpawnMode` (`self.SpawningMode`)
          (:`NewEnumerator0`
            ;[1 1 1] Single Type Per Wave
            ;;[1 1 1] Spawn loop
            (`KismetSystemLibrary.Delay` (`/Game/TowerDefense/Blueprints/Player/TD_GameMgnrActorComp.SpawnDelayGlobal` _returnvalue) :!label _label)
            (if (not _dontspawn)
              (`|SpawnActorFromClass` (`|GetArrayItem` _enemiestospawn (`/Game/TowerDefense/Blueprints/Player/TD_GameMgnrActorComp.SpawnIndex` _returnvalue)) (`self.GetTransform`) "Undefined" "MultiplyWithRoot" null null)
              ;;[1 1 1] Set enemy to spawn index
              (bind _output_get (set `self.LocalSpawnIndex` (+ (`self.LocalSpawnIndex`) 0)))
              (if (> _output_get (`KismetArrayLibrary.Array_Length` _enemiestospawn))
                (set `/Game/TowerDefense/Blueprints/Player/TD_GameMgnrActorComp.SpawnIndex` 0 _returnvalue) ; reset spawn index
                (goto _label)
                (else
                  (goto _label)))))
          (:`NewEnumerator1`
            ;[1 1 1] Random
            ;;[1 1 1] Spawn loop
            (`KismetSystemLibrary.Delay` (`/Game/TowerDefense/Blueprints/Player/TD_GameMgnrActorComp.SpawnDelayGlobal` _returnvalue) :!label _label_2)
            (if (not _dontspawn)
              (`|SpawnActorFromClass` (`|GetArrayItem` _enemiestospawn_2 (`KismetMathLibrary.RandomInteger` (`KismetArrayLibrary.Array_Length` _enemiestospawn_2))) (`self.GetTransform`) "Undefined" "MultiplyWithRoot" null null)
              (goto _label_2)))
          (:`NewEnumerator2`
            ;[1 1 1] One By One
            ;;[1 1 1] Spawn loop
            (`KismetSystemLibrary.Delay` (`/Game/TowerDefense/Blueprints/Player/TD_GameMgnrActorComp.SpawnDelayGlobal` _returnvalue) :!label _label_3)
            (if (not _dontspawn)
              (`|SpawnActorFromClass` (`|GetArrayItem` _enemiestospawn_3 (`self.LocalSpawnIndex`)) (`self.GetTransform`) "Undefined" "MultiplyWithRoot" null null)
              ;;[1 1 1] Set enemy to spawn index
              (bind _output_get_2 (set `self.LocalSpawnIndex` (+ (`self.LocalSpawnIndex`) 1)))
              (if (> _output_get_2 (`KismetArrayLibrary.Array_Length` _enemiestospawn_3))
                (set `self.LocalSpawnIndex` 0)
                (goto _label_3)
                (else
                  (goto _label_3))))))))))

(event `self.ReceiveBeginPlay`
  ;[1 1 1] Hide location cube
  (`SceneComponent.SetVisibility` (`self.LocationCube`) false false))

(fn `UserConstructionScript`)