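; PlayerBase is the tower defense base actor, which tracks its health and triggers the death screen when that health runs out.
; BeginPlay stores the starting health as the maximum, and AnyDamage subtracts incoming damage and prints the remaining health.
; Tick polls health and, once it reaches zero or below, uses a DoOnce to add a DeathMenu widget to the viewport a single time.
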(event `self.ReceiveBeginPlay`
  ;[1 1 1] Set Tag
  (set `self.Tags` (`self.Tags`))
  ;[1 1 1] Set Max HP
  (set `self.PlayerBaseHealthMax` (`self.PlayerBaseHealth`)))

(event `self.ReceiveAnyDamage`
  (params (Damage :type "Float (single-precision)") (DamageType :type "DamageType Object Reference") (InstigatedBy :type "Controller Object Reference") (DamageCauser :type "Actor Object Reference"))
  ;[1 1 1] Take Base Damage
  (`/Engine/EditorBlueprintResources/StandardMacros.DoOnce` false :!label _label
    (:`Completed`
      (bind _output_get (set `self.PlayerBaseHealth` (- (`self.PlayerBaseHealth`) Damage)))
      (`KismetSystemLibrary.PrintString` (`KismetStringLibrary.Conv_DoubleToString` _output_get))
      (goto _label :!via `Reset`))))

(event `self.ReceiveTick`
  (params (DeltaSeconds :type "Float (single-precision)"))
  ;[1 1 1] End Game If Base Health <= 0
  (if (<= (`self.PlayerBaseHealth`) 0.0)
    (`/Engine/EditorBlueprintResources/StandardMacros.DoOnce` false
      (:`Completed`
        ;[1 1 1] Add Death Menu
        (bind _returnvalue (`|CreateWidget` "/Game/TowerDefense/Blueprints/Widgets/DeathMenu.DeathMenu_C"))
        (`UserWidget.AddToViewport` _returnvalue 0)))))

(fn `UserConstructionScript`)